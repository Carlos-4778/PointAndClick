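; Base interactable item actor that the player can pick up, drop and inspect.
; Interacting attaches it to the player's ItemGrip with physics and collision off, or starts inspection if the player already holds an actor.
; Inspection swaps input from player to item and places it before the camera, where the mouse wheel changes distance and mouse movement rotates it while IsRotating.
; Interact ends inspection, resetting relative transform; DropItem detaches and restores physics.
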(event `InputAxisKey|MouseX`
  (params (AxisValue :type "Float (single-precision)"))
  (if (`self.IsRotating`)
    (`self.K2_SetActorRotation` (`KismetMathLibrary.ComposeRotators` (`self.K2_GetActorRotation`) (`KismetMathLibrary.MakeRotator` 0.0 0.0 (* AxisValue -5.0))))))

(event `/Game/InteractionSystem/IInteractable.InteractWith`
  (params (PlayerChar :type "/Game/FirstPersonCharacter Object Reference"))
  (bind _output_get (set `self.Player Char` PlayerChar))
  (`/Game/FirstPersonCharacter.CurrentlyHeldActor` _output_get
    (:`then`
      (`self.StartInspect`))
    (:`else`
      (`self.PickUpItem`))))

(event `InputAxisKey|MouseY`
  (params (AxisValue :type "Float (single-precision)"))
  (if (`self.IsRotating`)
    (`self.K2_SetActorRotation` (`KismetMathLibrary.ComposeRotators` (`self.K2_GetActorRotation`) (`KismetMathLibrary.MakeRotator` 0.0 (* AxisValue -5.0))))))

(event `InputAction|ActionInteract`
  (params (Key :type "Key Structure"))
  (:`Pressed`
    (`self.StopInspect`)))

(event `Key|MouseScrollUp`
  (params (Key :type "Key Structure"))
  (bind _returnvalue (`GameplayStatics.GetPlayerCameraManager` 0))
  (:`Pressed`
    (bind _output_get (set `self.ZoomLevel` (`KismetMathLibrary.Clamp` (+ (`self.ZoomLevel`) 1) 1 20)))
    (if (< _output_get 20)
      (`self.K2_SetActorLocation` (+ (`PlayerCameraManager.GetCameraLocation` _returnvalue) (* (`KismetMathLibrary.GetForwardVector` (`PlayerCameraManager.GetCameraRotation` _returnvalue)) (* (`self.ZoomLevel`) 20.0)))))))

(event `Key|MouseScrollDown`
  (params (Key :type "Key Structure"))
  (bind _returnvalue (`GameplayStatics.GetPlayerCameraManager` 0))
  (:`Pressed`
    (bind _output_get (set `self.ZoomLevel` (`KismetMathLibrary.Clamp` (- (`self.ZoomLevel`) 1) 1 20)))
    (if (> _output_get 1)
      (`self.K2_SetActorLocation` (+ (`PlayerCameraManager.GetCameraLocation` _returnvalue) (* (`KismetMathLibrary.GetForwardVector` (`PlayerCameraManager.GetCameraRotation` _returnvalue)) (* (`self.ZoomLevel`) 20.0)))))))

(fn `DropItem`
  (bind _returnvalue (`GameplayStatics.GetPlayerCameraManager` 0))
  (`self.K2_DetachFromActor` "KeepWorld" "KeepWorld" "KeepWorld")
  (`self.K2_SetActorLocation` (+ (`PlayerCameraManager.GetCameraLocation` _returnvalue) (* (`KismetMathLibrary.GetForwardVector` (`PlayerCameraManager.GetCameraRotation` _returnvalue)) 200.0)))
  (`PrimitiveComponent.SetSimulatePhysics` (`self.StaticMesh`) true)
  (`PrimitiveComponent.SetCollisionEnabled` (`self.StaticMesh`) "QueryAndPhysics"))

(fn `getInfos`
  (params (ObjectName :type Name))
  (returns (ObjectInfos :type "/Game/InteractionSystem/Datas/F_InteractableProps Structure"))
  (return))

(fn `PickUpItem`
  (`self.K2_AttachToComponent` (`/Game/FirstPersonCharacter.ItemGrip` (`self.Player Char`)) "None" "SnapToTarget" "SnapToTarget" "KeepRelative")
  (`PrimitiveComponent.SetSimulatePhysics` (`self.StaticMesh`) false)
  (`PrimitiveComponent.SetCollisionEnabled` (`self.StaticMesh`) "NoCollision")
  (set `/Game/FirstPersonCharacter.CurrentlyHeldActor` self (`self.Player Char`)))

(fn `StartInspect`
  (bind _returnvalue (`GameplayStatics.GetPlayerController` 0))
  (bind _returnvalue_2 (`GameplayStatics.GetPlayerCameraManager` 0))
  (`self.DisableInput` (`self.Player Char`) _returnvalue)
  (`self.EnableInput` _returnvalue)
  (`self.K2_SetActorLocation` (+ (`PlayerCameraManager.GetCameraLocation` _returnvalue_2) (* (`KismetMathLibrary.GetForwardVector` (`PlayerCameraManager.GetCameraRotation` _returnvalue_2)) 200.0))))

(fn `StopInspect`
  (bind _returnvalue (`GameplayStatics.GetPlayerController` 0))
  (`self.DisableInput` _returnvalue)
  (`self.EnableInput` (`self.Player Char`) _returnvalue)
  (`self.K2_SetActorRelativeLocation` (0.0 0.0 0.0))
  (`self.K2_SetActorRelativeRotation` (struct)))

(fn `UserConstructionScript`)