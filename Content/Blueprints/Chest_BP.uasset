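; Chest actor that the player pries open with a crowbar, with an inspectable mug spawned at it.
; BeginPlay spawns a FakeInspectMug_Child at the Billboard component's world location.
; Interactwith checks whether the player's held actor is the referenced Crowbar and, if so, destroys the chest's static mesh component.
; GetInfos is an empty stub.
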(event `self.ReceiveBeginPlay`
  (`|SpawnActorFromClass` "/Game/Blueprints/FakeInspectMug_Child.FakeInspectMug_Child_C" (`KismetMathLibrary.MakeTransform` (`SceneComponent.K2_GetComponentLocation` (`self.Billboard`))) "Undefined" "OverrideRootScale" null null))

(event `/Game/InteractionSystem/IInteractable.InteractWith`
  (params (PlayerChar :type "/Game/FirstPersonCharacter Object Reference"))
  (if (== (`/Game/FirstPersonCharacter.CurrentlyHeldActor` PlayerChar) (`self.Crowbar`))
    (`ActorComponent.K2_DestroyComponent` (`self.StaticMesh`))))

(fn `getInfos`
  (params (ObjectName :type Name))
  (returns (ObjectInfos :type "/Game/InteractionSystem/Datas/F_InteractableProps Structure"))
  (return))

(fn `UserConstructionScript`)