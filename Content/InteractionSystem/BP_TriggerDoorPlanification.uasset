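; BP_TriggerDoorPlanification is an interactable door trigger that teleports the first-person player once they have the Plani key.
; On Interact, it runs the parent logic, fades the camera out, moves the character to its Billboard's location and fades back in from black.
; A DoOnce blocks repeat triggers during the transition, then resets, re-enabling CanHoldItem if the player is not holding anything.
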(event `self.ReceiveBeginPlay`
  (bind _asfirst_person_character (cast `/Game/FirstPersonCharacter` (`GameplayStatics.GetPlayerCharacter` 0)))
  (set `self.As First Person Character` _asfirst_person_character))

(event `/Game/InteractionSystem/IInteractable.interact`
  (`parent.interact`)
  (if (`/Game/FirstPersonCharacter.HasPlaniKey?` (`self.As First Person Character`))
    (`/Engine/EditorBlueprintResources/StandardMacros.DoOnce` false :!label _label
      (:`Completed`
        (`PlayerCameraManager.StartCameraFade` :`self` (`GameplayStatics.GetPlayerCameraManager` 0) :`ToAlpha` 1.0 :`Duration` 1.5)
        (`KismetSystemLibrary.Delay` 1.5)
        (`self.K2_SetActorLocation` (`self.As First Person Character`) (`SceneComponent.K2_GetComponentLocation` (`self.Billboard`)) false false)
        (`PlayerCameraManager.StartCameraFade` (`GameplayStatics.GetPlayerCameraManager` 0) 1.0 0.0 1.5 (struct :`A` 1.0) false false)
        (if (`/Game/FirstPersonCharacter.IsHolding` (`self.As First Person Character`))
          (goto _label :!via `Reset`)
          (else
            (set `/Game/FirstPersonCharacter.CanHoldItem` true (`self.As First Person Character`))
            (goto _label :!via `Reset`)))))))

(fn `UserConstructionScript`
  (`parent.UserConstructionScript`))