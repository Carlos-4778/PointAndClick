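; BP_TriggerDoorOffice is an interactable door trigger that teleports the player when used.
; On BeginPlay it caches the player pawn as FirstPersonCharacter.
; Interact runs the parent interaction, then moves that character to the world location of the Billboard component, which serves as the destination marker, without sweeping.
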(event `self.ReceiveBeginPlay`
  (bind _asfirst_person_character (cast `/Game/FirstPersonCharacter` (`GameplayStatics.GetPlayerCharacter` 0)))
  (set `self.As First Person Character` _asfirst_person_character))

(event `/Game/InteractionSystem/IInteractable.interact`
  (`parent.interact`)
  (`self.K2_SetActorLocation` (`self.As First Person Character`) (`SceneComponent.K2_GetComponentLocation` (`self.Billboard`)) false false))

(fn `UserConstructionScript`
  (`parent.UserConstructionScript`))